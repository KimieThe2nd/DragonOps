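; Wyvern actor that flies a scripted two-leg route and destroys any actor that overlaps its Box component.
; Tick moves it continuously along its forward vector at WyvernSpeed without sweeping, so steering comes purely from rotation.
; After a short delay on BeginPlay, the FlightPath1 timeline drives that rotation.
; It then jumps to a hard-coded location, runs FlightPath2, and destroys itself when that finishes.
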(event `self.ReceiveTick`
  (params (DeltaSeconds :type "Float (single-precision)"))
  (`self.K2_AddActorWorldOffset` (* (* DeltaSeconds (`self.WyvernSpeed`)) (`KismetMathLibrary.GetForwardVector` (`self.K2_GetActorRotation`)))))

(event `self.ReceiveBeginPlay`
  (`KismetSystemLibrary.Delay` 3.0)
  (bind (_direction _rotation) (`Timeline|FlightPath1`)
    (:`Update`
      (`self.K2_SetActorRotation` (`KismetMathLibrary.MakeRotator` (.x _rotation) (.y _rotation) (.z _rotation))))
    (:`Finished`
      (`self.K2_SetActorLocation` (-10000.0 -1500.0 2000.0))
      (bind (_direction_2 _rotation_2) (`Timeline|FlightPath2`)
        (:`Update`
          (`self.K2_SetActorRotation` (`KismetMathLibrary.MakeRotator` (.x _rotation_2) (.y _rotation_2) (.z _rotation_2))))
        (:`Finished`
          (`self.K2_DestroyActor`))))))

(event `self.Box.OnComponentBeginOverlap`
  (params (OverlappedComponent :type "PrimitiveComponent Object Reference") (OtherActor :type "Actor Object Reference") (OtherComp :type "PrimitiveComponent Object Reference") (OtherBodyIndex :type Integer) (bFromSweep :type Boolean) (SweepResult :type "HitResult Structure (by ref)"))
  (`self.K2_DestroyActor` OtherActor))

(fn `UserConstructionScript`)