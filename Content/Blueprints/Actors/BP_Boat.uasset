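; BP_Boat is a boat actor that moves forward every tick and rocks side to side with a sine-driven roll.
; Its Gameify event plays a timeline that drives sound volume and low-pass cutoff.
; After a delay it switches the sound, turns off the filter, swaps the mesh to a pirate ship, resets speed and mesh position, and spawns two fish schools and a wyvern.
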(event `self.ReceiveTick`
  (params (DeltaSeconds :type "Float (single-precision)"))
  (set `self.Delta Seconds` DeltaSeconds)
  (`|ExecutionSequence`
    (:`then_0`
      ;[0 0 0] Boat Move
      (`self.K2_AddActorWorldOffset` (* (* (`self.Delta Seconds`) (`self.BoatSpeed`)) (`KismetMathLibrary.GetForwardVector` (`self.K2_GetActorRotation`)))))
    (:`then_1`
      ;[0 0 0] Boat Rock
      (`SceneComponent.K2_SetWorldRotation` (`self.DefaultSceneRoot`) (`KismetMathLibrary.MakeRotator` (* (`KismetMathLibrary.Sin` (* (`GameplayStatics.GetRealTimeSeconds`) (`self.BoatRockSpeed`))) (`self.BoatRockIntensity`))) false false))))

(event `/Game/Blueprints/Interfaces/BPI_Transform.Gameify`
  (bind _sound (`self.Sound`))
  (bind _returnvalue_x (`KismetMathLibrary.BreakVector` (`SceneComponent.K2_GetComponentLocation` (`self.BoatMesh`))))
  (bind _returnvalue_x_2 (`KismetMathLibrary.BreakVector` (`SceneComponent.K2_GetComponentLocation` (`self.BoatMesh`))))
  (`|ExecutionSequence`
    (:`then_0`
      (bind (_direction _volumemultiplier) (`Timeline|Timeline_0`)
        (:`Update`
          (`AudioComponent.SetVolumeMultiplier` (`self.Sound`) _volumemultiplier)
          (`AudioComponent.SetLowPassFilterFrequency` (`self.Sound`) (* _volumemultiplier 5000.0)))))
    (:`then_1`
      (`AudioComponent.SetLowPassFilterEnabled` (`self.Sound`) true)
      (`KismetSystemLibrary.Delay` 4.5)
      (`AudioComponent.SetSound` _sound "/Game/Sounds/Boat/Boat.Boat")
      (`AudioComponent.SetLowPassFilterEnabled` _sound false))
    (:`then_2`
      (`KismetSystemLibrary.Delay` 4.5)
      (`StaticMeshComponent.SetStaticMesh` (`self.BoatMesh`) "/Game/Meshes/PirateShip/AnyConv_com__PirateShip16.AnyConv_com__PirateShip16")
      (set `self.BoatSpeed` 100.0)
      (`SceneComponent.K2_SetRelativeLocation` (`self.BoatMesh`) (0.0 0.0 0.0) false false)
      (`|SpawnActorFromClass` "/Game/Blueprints/Actors/BP_FIshSchool.BP_FIshSchool_C" (`KismetMathLibrary.MakeTransform` (`KismetMathLibrary.MakeVector` (+ _returnvalue_x 1000.0) -1500.0 100.0)) "Undefined" "OverrideRootScale" null 25 true null)
      (`|SpawnActorFromClass` "/Game/Blueprints/Actors/BP_FIshSchool.BP_FIshSchool_C" (`KismetMathLibrary.MakeTransform` (`KismetMathLibrary.MakeVector` (+ _returnvalue_x_2 3000.0) 2000.0 100.0)) "Undefined" "OverrideRootScale" null 10 true null)
      (`|SpawnActorFromClass` "/Game/Blueprints/Actors/BP_Wyvern.BP_Wyvern_C" (`KismetMathLibrary.MakeTransform` (-437.0 -4931.0 4217.0) (struct :`Pitch` -24.268206 :`Yaw` 113.570987 :`Roll` 5.57232)) "Undefined" "OverrideRootScale" null null))))

(fn `UserConstructionScript`)