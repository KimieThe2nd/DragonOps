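; BP_Instance controls a background music track, exposing events to play, stop and adjust it.
; PlayAudio creates a 2D sound from Closed_Compartment that persists across level transitions without auto-destroying, stores it as Music and starts it.
; The other events act on that stored component to stop playback, set the volume multiplier, or toggle and tune a low-pass filter.
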(event `StopAudio`
  (`AudioComponent.Stop` (`self.Music`)))

(event `PlayAudio`
  (bind _returnvalue (`GameplayStatics.CreateSound2D` "/Game/Sounds/Music/Closed_Compartment.Closed_Compartment" 1.0 1.0 0.0 null true false))
  (bind _output_get (set `self.Music` _returnvalue))
  (`AudioComponent.Play` _output_get 0.0))

(event `SetMusicVolume`
  (params (VolumeMultiplier :type "Float (single-precision)"))
  (set `AudioComponent.VolumeMultiplier` VolumeMultiplier (`self.Music`)))

(event `SetMusicLowPassFilterEnabled`
  (params (LowPassFilterEnabled :type Boolean))
  (`AudioComponent.SetLowPassFilterEnabled` (`self.Music`) LowPassFilterEnabled))

(event `MusicSetLowPassFilterFrequency`
  (params (LowPassFilterFrequency :type "Float (single-precision)"))
  (`AudioComponent.SetLowPassFilterFrequency` (`self.Music`) LowPassFilterFrequency))