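; BP_FIshSchool is a spawner actor that populates the area around itself with a school of BP_Fish actors.
; SpawnSchool runs on BeginPlay when SpawnOnBeginPlay is set, looping from 2 to Amount to spawn fish.
; X is uniformly random around the root, while Y passes a random value through FishSpawnCurve to shape the distribution.
; All fish spawn at a fixed world height.
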(event `SpawnSchool`
  (params (Initiator :type "/Game/Blueprints/Actors/BP_Boat Object Reference"))
  (bind (_returnvalue_x _returnvalue_y) (`KismetMathLibrary.BreakVector` (`SceneComponent.K2_GetComponentLocation` (`self.DefaultSceneRoot`))))
  (for _ (range 2 (+ (`self.Amount`) 1))
    (`|SpawnActorFromClass` "/Game/Blueprints/Actors/BP_Fish.BP_Fish_C" (`KismetMathLibrary.MakeTransform` (`KismetMathLibrary.MakeVector` (`KismetMathLibrary.RandomFloatInRange` (- _returnvalue_x 1000.0) (+ _returnvalue_x 1000.0)) (`KismetMathLibrary.MapRangeClamped` (`CurveFloat.GetFloatValue` (`self.FishSpawnCurve`) (`KismetMathLibrary.RandomFloatInRange` -1.0 1.0)) -1.0 1.0 (- _returnvalue_y 1000.0) (+ _returnvalue_y 1000.0)) 40.0)) "Undefined" "OverrideRootScale" null null)))

(event `self.ReceiveBeginPlay`
  (if (`self.SpawnOnBeginPlay`)
    (`self.SpawnSchool` null)))

(fn `UserConstructionScript`)