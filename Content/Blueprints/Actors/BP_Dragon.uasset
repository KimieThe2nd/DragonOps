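; BP_Dragon is a dragon actor that flies continuously through the world and shakes nearby cameras.
; Each Tick it moves along its forward vector at DragonSpeed without sweeping and plays BP_DragonShake as a world camera shake centred on its location.
; A Timeline started on BeginPlay sets its rotation from a vector track, which steers the flight path.
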(event `self.ReceiveTick`
  (params (DeltaSeconds :type "Float (single-precision)"))
  (`self.K2_AddActorWorldOffset` (* (* DeltaSeconds (`self.DragonSpeed`)) (`KismetMathLibrary.GetForwardVector` (`self.K2_GetActorRotation`))))
  (`GameplayStatics.PlayWorldCameraShake` "/Game/Blueprints/CameraShakes/BP_DragonShake.BP_DragonShake_C" (`self.K2_GetActorLocation`) 10000.0 0.0 50.0 true))

(event `self.ReceiveBeginPlay`
  (bind (_direction _rotation) (`Timeline|Timeline`)
    (:`Update`
      (`self.K2_SetActorRotation` (`KismetMathLibrary.MakeRotator` (.x _rotation) (.y _rotation) (.z _rotation))))))

(fn `UserConstructionScript`)